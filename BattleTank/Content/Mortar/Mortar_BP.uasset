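; Mortar Blueprint, a turreted weapon actor with an aiming component and an on-screen health bar widget.
; On BeginPlay it initialises the TankAiming component with its turret and barrel meshes, reusing the tank's aiming setup.
; It then casts its HealthBar widget component's user widget and passes itself as the Tank so the bar can track it.
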(event EventBeginPlay
  (Class|TankAimingComponent|Initialise (Variables|Default|GetTankAiming) (Variables|Default|GetTankTurret) (Variables|Default|GetTankBarrel))
  (CallFunction|InitHealthBar))

(fn ConstructionScript)

(fn InitHealthBar
  (bind _ashealth_bar (Utilities|Casting|CastToHealthBar (UserInterface|GetUserWidgetObject (Variables|Default|GetHealthBarWidget))))
  (Variables|/Game/UI/HealthBar.HealthBar_C|SetTank _ashealth_bar self))